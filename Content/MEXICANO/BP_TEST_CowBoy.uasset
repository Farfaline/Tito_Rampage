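; BP_TEST_CowBoy is a test cowboy character Blueprint that cycles its eye expressions.
; On BeginPlay it creates a dynamic material instance on the second material slot of the CharaLoweye mesh.
; It then calls the Ded, OUCH and Classic events at timed intervals, each setting the material's "index" scalar parameter to switch the eye look.
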(event Custom|OUCH
  (Rendering|Material|SetScalarParameterValue (Variables|Default|Geteye_mat) "index" 1.0 :!class /Script/Engine.MaterialInstanceDynamic))

(event Custom|Ded
  (Rendering|Material|SetScalarParameterValue (Variables|Default|Geteye_mat) "index" -1.0 :!class /Script/Engine.MaterialInstanceDynamic))

(event Custom|Classic
  (Rendering|Material|SetScalarParameterValue (Variables|Default|Geteye_mat) "index" 0.0 :!class /Script/Engine.MaterialInstanceDynamic))

(event EventBeginPlay
  (bind _returnvalue (Rendering|Material|CreateDynamicMaterialInstance (Variables|Default|Getchara_low+eye) 1 (Rendering|Material|GetMaterial (Variables|Default|Getchara_low+eye) 1) "eyes" :!class /Script/Engine.PrimitiveComponent))
  (Variables|Default|Seteye_mat _returnvalue)
  (Utilities|FlowControl|Delay 3.0)
  (CallFunction|Ded)
  (Utilities|FlowControl|Delay 3.0)
  (CallFunction|OUCH)
  (Utilities|FlowControl|Delay 3.0)
  (CallFunction|Classic))

(fn ConstructionScript)